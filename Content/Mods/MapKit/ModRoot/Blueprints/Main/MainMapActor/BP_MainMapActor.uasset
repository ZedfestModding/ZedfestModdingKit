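; BP_MainMapActor is a map manager that sets up physics volumes and rotates enemy and boss spawn points between numbered map zones.
; On Tick it loads PhysicsVolumeLevel, diffs world actors to find new CustomVolume actors, then spawns AI spawn actors.
; After each ZoneTimer delay it cycles the zone, activates spawn points overlapping matching BP_MapZone cubes, and teleports spawned actors to active enemy points.
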(event `PrintToModLoader`
  (params (Message :type String)))

(event `self.ReceiveBeginPlay`
  (`SceneComponent.SetHiddenInGame` (`self.Plane`) true false)
  ;[0 0.08594 1] Check if this is actually needed later on
  (`KismetSystemLibrary.Delay` 1.0)
  (set `self.bInitalDelayFinished` true))

(event `self.ReceiveTick`
  (params (DeltaSeconds :type "Float (single-precision)"))
  (`self.StartPhysicsLogicLoading`)
  (`self.ZoneChange`))

(event `StartPhysicsLogicLoading`
  (if (not (`self.bHasFinishedWholeSetup`))
    (`self.PhysicsVolumeLevel`
      (:`then`
        (if (`LevelStreaming.IsLevelLoaded` (`self.PhysicsVolumeLevel`))
          (if (== 0 (`BlueprintMapLibrary.Map_Length` (`self.PhysicsVolume_InUse`)))
            (`self.TrimNewerActorList`)
            (else
              ;[1 0.1641 0] Not sure if this bool needs to be set before these two actually
              (set `self.bHasFinishedWholeSetup` true)
              (`self.GetMaxSpawnPointNumbers`)
              (`self.SpawnSpawnPoints`)))))
      (:`else`
        (`self.LoadPhysicsVolumeLevel`)))))

(event `TrimNewerActorList`
  (bind _outactors (`GameplayStatics.GetAllActorsOfClass` "/Script/Engine.Actor"))
  (set `self.NewerActorList` _outactors)
  (bind (_arrayindex _arrayelement) (`/Engine/EditorBlueprintResources/StandardMacros.ReverseForEachLoop` (`self.NewerActorList`))
    (:`LoopBody`
      (set `self.NewerActor` _arrayelement)
      (if (`KismetArrayLibrary.Array_Contains` (`self.ActorList`) (`self.NewerActor`))
        (`KismetArrayLibrary.Array_RemoveItem` (`self.NewerActorList`) (`self.NewerActor`))))
    (:`Completed`
      (`self.Make_PhysicsVolume_InUse_Map`))))

(event `Make_PhysicsVolume_InUse_Map`
  (for _array_element (`self.NewerActorList`)
    (set `self.NewerActor` _array_element)
    (`self.SetActorEnableCollision` (`self.NewerActor`) false)
    (if (`KismetStringLibrary.MatchesWildcard` (`KismetSystemLibrary.GetDisplayName` (`self.NewerActor`)) "*CustomVolume*")
      (`BlueprintMapLibrary.Map_Add` (`self.PhysicsVolume_InUse`) (`self.NewerActor`)))))

(event `LoadPhysicsVolumeLevel`
  (bind _outactors (`GameplayStatics.GetAllActorsOfClass` "/Script/Engine.Actor"))
  (set `self.ActorList` _outactors)
  (bind (_boutsuccess _returnvalue) (`LevelStreamingDynamic.LoadLevelInstance` "PhysicsVolumeLevel"))
  (set `self.PhysicsVolumeLevel` _returnvalue))

(event `ZoneChange`
  (if (`self.bHasHighestZoneNumber`)
    (if (`self.bHasInitializedAllSpawnPoints`)
      (`KismetSystemLibrary.Delay` (`self.ZoneTimer`))
      (`self.ChangeZoneNumber`)
      (`self.SetZoneSpawnPoints`)
      (`self.SetSpawnPointLocations`)
      (else
        (`self.SetZoneSpawnPoints`)
        (set `self.bHasInitializedAllSpawnPoints` true)))
    (else
      (`self.GetHighestZoneNumber`))))

(event `GetHighestZoneNumber`
  (bind _outactors (`GameplayStatics.GetAllActorsOfClass` "/Game/Mods/MapKit/ModRoot/Blueprints/Main/MapZones/BP_MapZone.BP_MapZone_C"))
  (for _array_element _outactors
    (bind _zonenumber (`/Game/Mods/MapKit/ModRoot/Blueprints/Main/MapZones/BP_MapZone.ZoneNumber` _array_element))
    (if (not (<= _zonenumber (`self.HighestZoneNumber`)))
      (set `self.HighestZoneNumber` _zonenumber)))
  (set `self.bHasHighestZoneNumber` true))

(event `ChangeZoneNumber`
  (if (== 0 (`self.HighestZoneNumber`))
    _
    (elif (== (`self.CurrentZoneNumber`) (`self.HighestZoneNumber`))
      (set `self.CurrentZoneNumber` 0)
      (else
        (set `self.CurrentZoneNumber` (+ 1 (`self.CurrentZoneNumber`)))))))

(event `SetZoneSpawnPoints`
  (bind _outactors (`GameplayStatics.GetAllActorsOfClass` "/Game/Mods/MapKit/ModRoot/Blueprints/Main/MapZones/BP_MapZone.BP_MapZone_C"))
  (for _array_element _outactors
    (set `self.ZoneOverlappedActors` (`PrimitiveComponent.GetOverlappingActors` (`/Game/Mods/MapKit/ModRoot/Blueprints/Main/MapZones/BP_MapZone.Cube` _array_element) "/Script/Engine.Actor"))
    (if (== (`/Game/Mods/MapKit/ModRoot/Blueprints/Main/MapZones/BP_MapZone.ZoneNumber` _array_element) (`self.CurrentZoneNumber`))
      (for _array_element_2 (`self.ZoneOverlappedActors`)
        (bind _asbp_enemy_spawn_point (cast `/Game/Mods/MapKit/ModRoot/Blueprints/Main/BP_EnemySpawnPoint` _array_element_2)
          (:`then`
            (set `/Game/Mods/MapKit/ModRoot/Blueprints/Main/BP_EnemySpawnPoint.bIsSpawnPointActive` true _asbp_enemy_spawn_point))
          (:`CastFailed`
            (bind _asbp_boss_spawn_point (cast `/Game/Mods/MapKit/ModRoot/Blueprints/Main/BP_BossSpawnPoint` _array_element_2))
            (set `/Game/Mods/MapKit/ModRoot/Blueprints/Main/BP_BossSpawnPoint.bIsSpawnPointActive` true _asbp_boss_spawn_point))))
      (else
        (for _array_element_3 (`self.ZoneOverlappedActors`)
          (bind _asbp_enemy_spawn_point_2 (cast `/Game/Mods/MapKit/ModRoot/Blueprints/Main/BP_EnemySpawnPoint` _array_element_3)
            (:`then`
              (set `/Game/Mods/MapKit/ModRoot/Blueprints/Main/BP_EnemySpawnPoint.bIsSpawnPointActive` false _asbp_enemy_spawn_point_2))
            (:`CastFailed`
              (bind _asbp_boss_spawn_point_2 (cast `/Game/Mods/MapKit/ModRoot/Blueprints/Main/BP_BossSpawnPoint` _array_element_3))
              (set `/Game/Mods/MapKit/ModRoot/Blueprints/Main/BP_BossSpawnPoint.bIsSpawnPointActive` false _asbp_boss_spawn_point_2))))))))

(event `GetMaxSpawnPointNumbers`
  (bind _outactors (`GameplayStatics.GetAllActorsOfClass` "/Game/Mods/MapKit/ModRoot/Blueprints/Main/MapZones/BP_MapZone.BP_MapZone_C"))
  (for _array_element _outactors
    (for _array_element_2 (`PrimitiveComponent.GetOverlappingActors` (`/Game/Mods/MapKit/ModRoot/Blueprints/Main/MapZones/BP_MapZone.Cube` _array_element) "/Script/Engine.Actor")
      (cast `/Game/Mods/MapKit/ModRoot/Blueprints/Main/BP_EnemySpawnPoint` _array_element_2)
      (set `self.TempHighestEnemySpawnPointNumber` (+ 1 (`self.TempHighestEnemySpawnPointNumber`))))))

(event `SetSpawnPointLocations`
  (`KismetArrayLibrary.Array_Clear` (`self.ActiveEnemySpawnPoints`))
  (bind _outactors (`GameplayStatics.GetAllActorsOfClass` "/Game/Mods/MapKit/ModRoot/Blueprints/Main/BP_EnemySpawnPoint.BP_EnemySpawnPoint_C"))
  (for _array_element _outactors
    (if (`/Game/Mods/MapKit/ModRoot/Blueprints/Main/BP_EnemySpawnPoint.bIsSpawnPointActive` _array_element)
      (`KismetArrayLibrary.Array_AddUnique` (`self.ActiveEnemySpawnPoints`) _array_element)))
  (for _array_element_2 (`self.EnemySpawnPoints`)
    (set `self.EnemySpawnPoint` _array_element_2)
    (set `self.EnemyActiveSpawnPoint` (`|GetArrayItem` (`self.ActiveEnemySpawnPoints`) (`self.EnemySpawnPointCounter`)) :!label _label)
    (`self.EnemyActiveSpawnPoint`
      (:`then`
        (`self.K2_SetActorLocation` (`self.EnemySpawnPoint`) (`self.K2_GetActorLocation` (`self.EnemyActiveSpawnPoint`)) false true))
      (:`else`
        (set `self.EnemySpawnPointCounter` 0)
        (goto _label)))))

(event `SpawnSpawnPoints`
  (if (not (== (`KismetArrayLibrary.Array_Length` (`self.EnemySpawnPoints`)) (`self.HighestEnemySpawnPointNumber`))) :!label _label_2
    (bind _returnvalue (`|SpawnActorFromClass` "/Game/HordeTemplateBP/Blueprint/Ai/BP_Base_AI_SpawnExpand.BP_Base_AI_SpawnExpand_C" (`KismetMathLibrary.MakeTransform` (0.0 0.0 0.0)) "AdjustIfPossibleButAlwaysSpawn" "OverrideRootScale" null null))
    (`KismetArrayLibrary.Array_AddUnique` (`self.EnemySpawnPoints`) _returnvalue)
    (goto _label_2)))

(fn `UserConstructionScript`)