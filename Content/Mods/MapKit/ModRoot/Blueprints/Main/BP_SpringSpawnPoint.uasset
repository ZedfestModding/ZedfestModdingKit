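; BP_SpringSpawnPoint is a map kit spawn point that creates a BP_Spring aimed at a landing target.
; BeginPlay hides its components and spawns a temporary spring without a target.
; After a shared delay, it spawns a BP_TargetPoint at the LandingPoint offset, replacing the temporary spring with one linked to that target's billboard.
; Once spawned, Tick keeps reassigning the target to the spring.
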(event `self.ReceiveTick`
  (params (DeltaSeconds :type "Float (single-precision)"))
  (if (`self.bHasSpawned`)
    (set `/Game/Blueprints/GenericShooter/Addons/Interaction/Examples/BonusContent/Spring/BP_Spring.TargetPoint` (`self.TargetPoint`) (`self.BP_Spring`))
    (else
      (`KismetSystemLibrary.Delay` 3.0 :!label _label)
      (bind _returnvalue (`|SpawnActorFromClass` "/Game/Mods/MapKit/ModRoot/Blueprints/Other/BP_TargetPoint.BP_TargetPoint_C" (`KismetMathLibrary.MakeTransform` (+ (`self.K2_GetActorLocation`) (`self.LandingPoint`))) "AlwaysSpawn" "OverrideRootScale" null null))
      (bind _output_get (set `self.TargetPoint` (`/Game/Mods/MapKit/ModRoot/Blueprints/Other/BP_TargetPoint.BillboardTargetPoint` _returnvalue)))
      (bind _returnvalue_2 (`|SpawnActorFromClass` "/Game/Blueprints/GenericShooter/Addons/Interaction/Examples/BonusContent/Spring/BP_Spring.BP_Spring_C" (`self.GetTransform`) "AlwaysSpawn" "OverrideRootScale" null _output_get null))
      (set `self.BP_Spring` _returnvalue_2)
      (`self.K2_DestroyActor` (stale `self.ReceiveBeginPlay` _returnvalue))
      (set `self.bHasSpawned` true))))

(event `self.ReceiveBeginPlay`
  (`SceneComponent.SetHiddenInGame` (`self.DefaultSceneRoot`) true true)
  (bind _returnvalue (`|SpawnActorFromClass` "/Game/Blueprints/GenericShooter/Addons/Interaction/Examples/BonusContent/Spring/BP_Spring.BP_Spring_C" (`self.GetTransform`) "AlwaysSpawn" "OverrideRootScale" null null null))
  (goto _label))

(fn `UserConstructionScript`)