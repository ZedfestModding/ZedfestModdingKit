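; Map-kit swimming zone that gives overlapping actors a pooled physics volume so they can swim inside its Cube.
; On BeginPlay it spawns a scaled-down BP_Water and copies its mesh material onto the Cube.
; Overlap start checks the pawn's attachments for a "CustomVolume", claims free volumes from BP_MainMapActor's in-use map, then attaches one with collision enabled.
; Overlap end marks the last-used volume free and disables its collision without detaching it.
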(event `self.ReceiveBeginPlay`
  (bind (_returnvalue_location _returnvalue_rotation _returnvalue_scale) (`KismetMathLibrary.BreakTransform` (`self.GetTransform`)))
  (bind _returnvalue (`|SpawnActorFromClass` "/Game/Meshes/ISW/Blueprint/BP_Water.BP_Water_C" (`KismetMathLibrary.MakeTransform` _returnvalue_location _returnvalue_rotation (* _returnvalue_scale 0.2)) "AlwaysSpawn" "OverrideRootScale" null null))
  (for _array_element (`self.K2_GetComponentsByClass` _returnvalue "/Script/Engine.MeshComponent")
    (`PrimitiveComponent.SetMaterial` (`self.Cube`) 0 (`PrimitiveComponent.GetMaterial` _array_element 0))))

(event `self.Cube.OnComponentBeginOverlap`
  (params (OverlappedComponent :type "PrimitiveComponent Object Reference") (OtherActor :type "Actor Object Reference") (OtherComp :type "PrimitiveComponent Object Reference") (OtherBodyIndex :type Integer) (bFromSweep :type Boolean) (SweepResult :type "HitResult Structure (by ref)"))
  (set `self.OverlappedActor` OtherActor)
  (`self.StartSwimming`))

(event `self.Cube.OnComponentEndOverlap`
  (params (OverlappedComponent :type "PrimitiveComponent Object Reference") (OtherActor :type "Actor Object Reference") (OtherComp :type "PrimitiveComponent Object Reference") (OtherBodyIndex :type Integer))
  (set `self.OverlappedActor` OtherActor)
  (`self.EndSwimming`))

(event `StartSwimming`
  (`self.Get_PhysicsVolume_InUse_Map`)
  (for _array_element (`self.GetAttachedActors` (cast `/Game/NetworkRagdollIK/Blueprints/BP_Pawn` (`self.OverlappedActor`) :!pure true))
    (set `self.AttachedActor` _array_element)
    (if (`KismetStringLibrary.MatchesWildcard` (`KismetSystemLibrary.GetDisplayName` (`self.AttachedActor`)) "*CustomVolume*")
      (set `self.PhysicsVolumeActor` (`self.AttachedActor`))
      (break)
      (else
        (bind _keys (`BlueprintMapLibrary.Map_Keys` (`self.PhysicsVolume_InUse_Map`)))
        (for _array_element_2 _keys
          (set `self.PhysicsObject` _array_element_2)
          (if (== false (`BlueprintMapLibrary.Map_Find` (`self.PhysicsVolume_InUse_Map`) (`self.PhysicsObject`)))
            (`BlueprintMapLibrary.Map_Remove` (`self.PhysicsVolume_InUse_Map`) (`self.PhysicsObject`))
            (`BlueprintMapLibrary.Map_Add` (`self.PhysicsVolume_InUse_Map`) (`self.PhysicsObject`) true)
            (break))))))
  (`self.AttachPhysicsVolume`))

(event `EndSwimming`
  (`BlueprintMapLibrary.Map_Remove` (`self.PhysicsVolume_InUse_Map`) (`self.PhysicsObject`))
  (`BlueprintMapLibrary.Map_Add` (`self.PhysicsVolume_InUse_Map`) (`self.PhysicsObject`))
  (bind _asactor (cast `Actor` (`self.PhysicsObject`)))
  (`self.SetActorEnableCollision` _asactor false))

(event `Get_PhysicsVolume_InUse_Map`
  (`self.MainVolumeActor`
    (:`then`
      _)
    (:`else`
      (bind _outactors (`GameplayStatics.GetAllActorsOfClass` "/Game/Mods/MapKit/ModRoot/Blueprints/Main/MainMapActor/BP_MainMapActor.BP_MainMapActor_C"))
      (set `self.MainVolumeActor` (`|GetArrayItem` _outactors))))
  (set `self.PhysicsVolume_InUse_Map` (`/Game/Mods/MapKit/ModRoot/Blueprints/Main/MainMapActor/BP_MainMapActor.PhysicsVolume_InUse` (`self.MainVolumeActor`))))

(event `AttachPhysicsVolume`
  (set `self.PhysicsVolume` (cast `Actor` (`self.PhysicsObject`) :!pure true))
  (`self.SetActorEnableCollision` (`self.PhysicsVolume`) true)
  (`self.K2_AttachToActor` (`self.PhysicsVolume`) (`self.OverlappedActor`) "None" "SnapToTarget" "SnapToTarget" "SnapToTarget" true))

(fn `UserConstructionScript`)