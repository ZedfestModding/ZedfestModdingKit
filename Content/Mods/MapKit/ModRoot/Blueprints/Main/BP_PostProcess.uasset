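; MapKit mod actor that adds post-processing to the world by loading PostProcessVolumeLevel as a level instance at the origin on BeginPlay.
; Tick also serves as a debug hook, printing the names of all user widgets when the 4 key is pressed.
; Unconnected leftover logic streams Level_Demonstration and diffs actor snapshots to destroy all new actors except PostProcessVolumes, or loads another post-process level at the player's location.
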(event `self.ReceiveBeginPlay`
  (`LevelStreamingDynamic.LoadLevelInstance` "/Game/Mods/Z_Mapping_P/ModRoot/Levels/PostProcessVolumeLevel"))

(event `self.ReceiveTick`
  (params (DeltaSeconds :type "Float (single-precision)"))
  (if (`PlayerController.WasInputKeyJustPressed` (`GameplayStatics.GetPlayerController` 0) "Four")
    (bind _foundwidgets (`WidgetBlueprintLibrary.GetAllWidgetsOfClass` "/Script/UMG.UserWidget" false))
    (for _array_element _foundwidgets
      (`self.ModPrint` (`KismetSystemLibrary.GetDisplayName` _array_element)))))

(fn `LocalPrintToModLoader`
  (params (InputMessage :type String))
  (`self.ModActor`
    (:`then`
      _)
    (:`else`
      (bind _outactors (`GameplayStatics.GetAllActorsOfClass` "/Game/Mods/MapKit/ModRoot/Blueprints/Other/Z_Debugging_P/ModActor.ModActor_C"))
      (set `self.ModActor` (`|GetArrayItem` _outactors))))
  (`/Game/Mods/MapKit/ModRoot/Blueprints/Other/Z_Debugging_P/ModActor.PrintToModLoader` (`self.ModActor`) (`local.InputMessage`)))

(fn `UserConstructionScript`)