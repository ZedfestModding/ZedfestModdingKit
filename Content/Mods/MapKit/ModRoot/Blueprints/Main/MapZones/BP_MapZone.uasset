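; BP_MapZone is a numbered map zone volume that damages players inside it whenever it is not the current zone.
; On tick it finds or spawns BP_MainMapActor and compares its CurrentZoneNumber to its own, switching the cube between translucent (safe) and red (damaging).
; A tick-driven Delay paces point damage to overlapping pawns by DamageDelay.
; The construction script sets the mesh and colors the cube by zone number.
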(event `self.ReceiveTick`
  (params (DeltaSeconds :type "Float (single-precision)"))
  (`self.MaintainReferences`)
  (`self.SetCubeMaterial`)
  (`self.ZoneCheck`))

(event `MaintainReferences`
  (`self.MainModActor`
    (:`then`
      _)
    (:`else`
      (bind _outactors (`GameplayStatics.GetAllActorsOfClass` "/Game/Mods/MapKit/ModRoot/Blueprints/Main/MainMapActor/BP_MainMapActor.BP_MainMapActor_C"))
      (set `self.MainModActor` (`|GetArrayItem` _outactors))))
  (`self.MainModActor`
    (:`then`)
    (:`else`
      (bind _returnvalue (`|SpawnActorFromClass` "/Game/Mods/MapKit/ModRoot/Blueprints/Main/MainMapActor/BP_MainMapActor.BP_MainMapActor_C" (`KismetMathLibrary.MakeTransform` (0.0 0.0 0.0)) "AdjustIfPossibleButAlwaysSpawn" "OverrideRootScale" null null))
      (set `self.MainModActor` _returnvalue))))

(event `SetCubeMaterial`
  (if (== (`/Game/Mods/MapKit/ModRoot/Blueprints/Main/MainMapActor/BP_MainMapActor.CurrentZoneNumber` (`self.MainModActor`)) (`self.ZoneNumber`))
    (`PrimitiveComponent.SetMaterial` (`self.Cube`) 0 "/Game/Mods/MapKit/ModRoot/Materials/M_Translucent.M_Translucent")
    (set `self.bDamagePlayer` false)
    (else
      (`PrimitiveComponent.SetMaterial` (`self.Cube`) 0 "/Game/Mods/MapKit/ModRoot/Blueprints/Main/MapZones/Materials/MI_MapZoneRed.MI_MapZoneRed")
      (set `self.bDamagePlayer` true))))

(event `ZoneCheck`
  (`KismetSystemLibrary.Delay` (`self.DamageDelay`))
  (for _array_element (`PrimitiveComponent.GetOverlappingActors` (`self.Cube`) (`GameplayStatics.GetObjectClass` (`GameplayStatics.GetPlayerPawn` 0)))
    (bind _asbp_pawn (cast `/Game/NetworkRagdollIK/Blueprints/BP_Pawn` _array_element))
    (if (`self.bDamagePlayer`)
      (`GameplayStatics.ApplyPointDamage` _asbp_pawn (`self.DamageAmount`) (`self.HitFromDirection`) (`self.HitInfo`) null null "/Game/HordeTemplateBP/Blueprint/Base/BP_Damage_Player.BP_Damage_Player_C"))))

(fn `UserConstructionScript`
  (set `self.ZoneMaterials` (`|MakeArray` "/Game/Mods/MapKit/ModRoot/Blueprints/Main/MapZones/Materials/MI_MapZoneBlack.MI_MapZoneBlack" "/Game/Mods/MapKit/ModRoot/Blueprints/Main/MapZones/Materials/MI_MapZoneBlue.MI_MapZoneBlue" "/Game/Mods/MapKit/ModRoot/Blueprints/Main/MapZones/Materials/MI_MapZoneGreen.MI_MapZoneGreen" "/Game/Mods/MapKit/ModRoot/Blueprints/Main/MapZones/Materials/MI_MapZoneOrange.MI_MapZoneOrange" "/Game/Mods/MapKit/ModRoot/Blueprints/Main/MapZones/Materials/MI_MapZonePurple.MI_MapZonePurple" "/Game/Mods/MapKit/ModRoot/Blueprints/Main/MapZones/Materials/MI_MapZoneRed.MI_MapZoneRed" "/Game/Mods/MapKit/ModRoot/Blueprints/Main/MapZones/Materials/MI_MapZoneWhite.MI_MapZoneWhite" "/Game/Mods/MapKit/ModRoot/Blueprints/Main/MapZones/Materials/MI_MapZoneYellow.MI_MapZoneYellow" "/Game/Mods/MapKit/ModRoot/Blueprints/Main/MapZones/Materials/MI_MapZoneGrey.MI_MapZoneGrey" :!type "MaterialInstance Object Reference"))
  (`StaticMeshComponent.SetStaticMesh` (`self.Cube`) (`self.StaticMesh`))
  (set `self.Material` (`|GetArrayItem` (`self.ZoneMaterials`) (`self.ZoneNumber`)))
  (`PrimitiveComponent.SetMaterial` (`self.Cube`) 0 (`self.Material`)))