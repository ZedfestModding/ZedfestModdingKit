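; BP_MapLoader is a MapKit mod Blueprint that registers custom maps in the game's level menu at BeginPlay.
; It force-scans /Game/Mods through the Asset Registry, polling until loading finishes, then walks every DataTable asset in reverse order.
; Each row becomes a PlayableLevels entry added uniquely to BP_Horde_Instance's AvailableLevels, with a shared transition map.
; A LevelName comparison keeps a developer-only map out of the menu.
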(event `self.ReceiveBeginPlay`
  (`AssetRegistry.ScanPathsSynchronous` (`AssetRegistryHelpers.GetAssetRegistry`) (`|MakeArray` "/Game/Mods") true)
  (if (`AssetRegistry.IsLoadingAssets` (`AssetRegistryHelpers.GetAssetRegistry`)) :!label _label
    (`KismetSystemLibrary.Delay` 0.1)
    (goto _label)
    (else
      (bind (_arrayindex _arrayelement) (`/Engine/EditorBlueprintResources/StandardMacros.ReverseForEachLoop` (`AssetRegistry.GetAssetsByClass` (`AssetRegistryHelpers.GetAssetRegistry`) "DataTable" false))
        (:`LoopBody`
          (bind _asdata_table (cast `DataTable` (`AssetRegistryHelpers.GetAsset` _arrayelement) :!pure true))
          (bind _outrownames (`DataTableFunctionLibrary.GetDataTableRowNames` _asdata_table))
          (for _array_element _outrownames
            (bind _returnvalue (`|GetDataTableRow` _asdata_table _array_element)
              (:`then`
                (bind (_level_name _level_image _level_raw_name _level_description) (break `/Game/Mods/MapKit/ModRoot/Structs/F_AddMapToMenu` _returnvalue))
                ;[1 0 0.7031] Prevents a developer only map from being added to the menu
                (if (not (`KismetTextLibrary.EqualEqual_TextText` _level_name (`self.ComparisonText`)))
                  (`KismetArrayLibrary.Array_AddUnique` (`/Game/HordeTemplateBP/Blueprint/Base/BP_Horde_Instance.AvailableLevels` (cast `/Game/HordeTemplateBP/Blueprint/Base/BP_Horde_Instance` (`GameplayStatics.GetGameInstance`) :!pure true)) (make `/Game/HordeTemplateBP/Blueprint/Struct/PlayableLevels` _level_name _level_image _level_raw_name _level_description "TransitionMap")))))))))))

(fn `ActivateConsole`)

(fn `UserConstructionScript`)