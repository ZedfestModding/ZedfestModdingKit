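; Debugging module for the mod loader, offering developer test actions and an instant game quit on the Pause key.
; Mod button presses dispatch by index to world speed toggling, looked-at actor destruction, a PDA_ModLoader asset scan, pak mounting or a main menu widget.
; The pak test chains mobile-patching content request, install and mount, printing failures and mount status through ModPrint.
; Several print helpers and unwired experiments remain as scratch code.
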(event `self.ReceiveTick`
  (params (DeltaSeconds :type "Float (single-precision)"))
  (if (`PlayerController.WasInputKeyJustPressed` (`GameplayStatics.GetPlayerController` 0) "Pause")
    (`KismetSystemLibrary.QuitGame` null "Quit")))

(event `self.ModButtonWasPressed`
  (params (FunctionIndex :type Integer))
  (switch `int` FunctionIndex
    (:`0`
      (`/Game/Mods/ModLoader/ModRoot/Modules/Debugging/BFL_Debugging.ToggleWorldSpeedChange`))
    (:`1`
      (`/Game/Mods/ModLoader/ModRoot/Modules/Debugging/BFL_Debugging.DestroyActorLookingAt`))
    (:`2`
      (`self.TestPrimaryAssetLabel`))
    (:`3`
      (`self.PakMountingTesting`))
    (:`4`
      (`self.MenuTest`))))

(event `self.ReceiveBeginPlay`)

(event `MenuTest`
  (bind _returnvalue (`|CreateWidget` "/Game/Mods/ModLoader/ModRoot/NewMenu/Widgets/WBP_MainMenu.WBP_MainMenu_C"))
  (`UserWidget.AddToViewport` _returnvalue 100))

(event `TestPrimaryAssetLabel`
  (for _array_element (`AssetRegistry.GetAssetsByClass` (`AssetRegistryHelpers.GetAssetRegistry`) "PrimaryDataAsset" true)
    (bind _aspda_mod_loader (cast `/Game/Mods/ModLoader/ModRoot/Shared/Bases/PDA_ModLoader` (`AssetRegistryHelpers.GetAsset` _array_element)))
    (for _ (`/Game/Mods/ModLoader/ModRoot/Shared/Bases/PDA_ModLoader.ModLoaderInformation` _aspda_mod_loader)
      _)))

(event `PakMountingTesting`
  (`MobilePatchingLibrary.RequestContent` (`self.RemoteManifestURL`) (`self.CloudURL`) (`self.InstallDirectory`) (delegate `RequestContentEventPassed`) (delegate `RequestContentEventFailed`)))

(event `RequestContentEventPassed`
  (params (MobilePendingContent :type "MobilePendingContent Object Reference"))
  (bind _output_get (set `self.MobilePendingContent` MobilePendingContent))
  (`MobilePendingContent.StartInstall` _output_get (delegate `InstallEventPassed`) (delegate `InstallEventFailed`)))

(event `RequestContentEventFailed`
  (params (ErrorText :type Text) (ErrorCode :type Integer))
  (`/Game/Mods/ModLoader/ModRoot/Modules/Logging/BFL_DebugLog.ModPrint` (`KismetTextLibrary.Conv_TextToString` ErrorText)))

(event `InstallEventPassed`
  (`self.MountContent`))

(event `InstallEventFailed`
  (params (ErrorText :type Text) (ErrorCode :type Integer))
  (`/Game/Mods/ModLoader/ModRoot/Modules/Logging/BFL_DebugLog.ModPrint` (`KismetTextLibrary.Conv_TextToString` ErrorText)))

(event `MountContent`
  (bind _returnvalue (`MobileInstalledContent.Mount` (`MobilePatchingLibrary.GetInstalledContent` (`self.InstallDirectory`)) 1 ""))
  (`/Game/Mods/ModLoader/ModRoot/Modules/Logging/BFL_DebugLog.ModPrint` (`KismetStringLibrary.Concat_StrStr` "Content Mount Status: " (`KismetStringLibrary.Conv_BoolToString` _returnvalue))))

(fn `CollectGarbage`
  (`self.CollectGarbage`))

(fn `FancyPrintTest`
  (`/Game/Mods/ModLoader/ModRoot/Modules/Logging/BFL_DebugLog.ModPrintFancyArray` (`|MakeArray` "Test 1" "Test 2" "Test 3" "Test 4") true false "" (struct :`R` 0.211765 :`G` 0.086275 :`B` 0.019608 :`A` 1.0) (make `SlateColor` (struct :`G` 0.061501 :`B` 1.0 :`A` 1.0)) (make `SlateFontInfo` null null (struct :`OutlineColor` (struct :`A` 1.0)) "Light" 12) (struct :`R` 0.152941 :`G` 0.054902 :`A` 1.0) (make `SlateColor` (struct :`R` 0.437617 :`G` 1.0 :`A` 1.0)) (make `SlateFontInfo` null null (struct :`OutlineColor` (struct :`A` 1.0)) "Light" 12))
  (bind _outactors (`GameplayStatics.GetAllActorsOfClass` "/Game/Mods/ModLoader/ModRoot/Modules/ModLoader/BP_ModLoader.BP_ModLoader_C"))
  (`/Game/Mods/ModLoader/ModRoot/Modules/Logging/BFL_DebugLog.ModPrint` (`KismetStringLibrary.Conv_IntToString` (`KismetArrayLibrary.Array_Length` _outactors)) true)
  (bind _modloaderinformation (`/Game/Mods/ModLoader/ModRoot/Modules/ModLoader/BP_ModLoader.ModLoaderInformation` (`|GetArrayItem` _outactors)))
  (`/Game/Mods/ModLoader/ModRoot/Modules/Logging/BFL_DebugLog.ModPrint` (`KismetStringLibrary.Conv_IntToString` (`KismetArrayLibrary.Array_Length` _modloaderinformation)) true)
  (for _array_element _modloaderinformation
    (`/Game/Mods/ModLoader/ModRoot/Modules/Logging/BFL_DebugLog.ModPrint` (`.ModName_2_508F97D64480667C0B029280456ECDF8` (break `/Game/Mods/ModLoader/ModRoot/Modules/ModLoader/F_ModLoaderInformation` _array_element)))))

(fn `PrintGameInformation`
  (`/Game/Mods/ModLoader/ModRoot/Modules/Logging/BFL_DebugLog.ModPrint` "Current Level:")
  (bind _returnvalue (`GameplayStatics.GetCurrentLevelName` true))
  (`/Game/Mods/ModLoader/ModRoot/Modules/Logging/BFL_DebugLog.ModPrint` _returnvalue true))

(fn `TestingFunction`)

(fn `UserConstructionScript`
  (`parent.UserConstructionScript`))