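; BP_Main_Themes is the Themes module Blueprint in the mod loader, currently an unfinished stub.
; BeginPlay runs InBetweenLogic, which calls an empty LoadThemeDataAsset event, then calls the parent BeginPlay.
; A disconnected chain blocking-loads the default themes data asset, casts it to PDA_Themes and loops over its Themes with an empty body, so no themes are loaded at runtime here.
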(event `self.ReceiveBeginPlay`
  (`self.InBetweenLogic`)
  (`parent.ReceiveBeginPlay`))

(event `InBetweenLogic`
  (`self.LoadThemeDataAsset`))

(event `LoadThemeDataAsset`)

(fn `UserConstructionScript`
  (`parent.UserConstructionScript`))