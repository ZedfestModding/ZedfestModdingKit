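; Mod loader actor that finds and spawns mods and toggles the WBP_ModLoader menu by key press.
; Its construction script loads SG_ModTracker, rescans /Game/Mods, then spawns listed mods, currently ignoring their active flag.
; A DataTable selects discovery: primary data assets, data tables or ModActor naming, with level streaming and console-command spawn variants.
; Data asset and table scans merge saved per-mod settings before cleanup and saving.
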(event `PrintToModLoader`
  (params (Message :type String)))

(event `SpawnLogicModsLevelStreamMethod`
  (bind _modsdir (`self.ModsDir`))
  (for _array_element (`AssetRegistry.GetAllCachedPaths` (`AssetRegistryHelpers.GetAssetRegistry`))
    (if (`KismetStringLibrary.StartsWith` _array_element (`self.ModsDir`))
      (if (not (`KismetStringLibrary.EndsWith` _array_element "/"))
        (bind _returnvalue (`KismetSystemLibrary.LoadAsset_Blocking` (`KismetSystemLibrary.Conv_SoftObjPathToSoftObjRef` (`KismetSystemLibrary.MakeSoftObjectPath` (`KismetStringLibrary.Concat_StrStr` _array_element "/ModActor.ModActor_C")))))
        (if (`KismetSystemLibrary.IsValid` _returnvalue)
          (bind _returnvalue_2 (`KismetStringLibrary.RightChop` _array_element (`KismetStringLibrary.Len` _modsdir)))
          (bind _returnvalue_3 (`KismetStringLibrary.Concat_StrStr` _modsdir _returnvalue_2 "/" _returnvalue_2 "Level"))
          (`/Game/Mods/ModLoader/ModRoot/Modules/Logging/BFL_DebugLog.ModPrint` _returnvalue_3)
          (`LevelStreamingDynamic.LoadLevelInstance` _returnvalue_3))))))

(event `SpawnLogicModsSpawnActorMethodSummon`
  (for _array_element (`AssetRegistry.GetAllCachedPaths` (`AssetRegistryHelpers.GetAssetRegistry`))
    (if (`KismetStringLibrary.StartsWith` _array_element (`self.ModsDir`))
      (if (not (`KismetStringLibrary.EndsWith` _array_element "/"))
        (bind _returnvalue (`KismetSystemLibrary.LoadAsset_Blocking` (`KismetSystemLibrary.Conv_SoftObjPathToSoftObjRef` (`KismetSystemLibrary.MakeSoftObjectPath` (`KismetStringLibrary.Concat_StrStr` _array_element "/ModActor.ModActor_C")))))
        (if (`KismetSystemLibrary.IsValid` _returnvalue)
          (if (`KismetSystemLibrary.IsValidClass` (`GameplayStatics.GetObjectClass` _returnvalue))
            (`KismetSystemLibrary.ExecuteConsoleCommand` "enablecheats" null)
            (`KismetSystemLibrary.ExecuteConsoleCommand` (`KismetStringLibrary.Concat_StrStr` "summon " (`KismetStringLibrary.Concat_StrStr` _array_element "/ModActor")) null)))))))

(event `SpawnLogicModsSpawnActorMethodSpawnActor`
  (for _array_element (`AssetRegistry.GetAllCachedPaths` (`AssetRegistryHelpers.GetAssetRegistry`))
    (if (`KismetStringLibrary.StartsWith` _array_element (`self.ModsDir`))
      (if (not (`KismetStringLibrary.EndsWith` _array_element "/"))
        (bind _returnvalue (`KismetSystemLibrary.LoadAsset_Blocking` (`KismetSystemLibrary.Conv_SoftObjPathToSoftObjRef` (`KismetSystemLibrary.MakeSoftObjectPath` (`KismetStringLibrary.Concat_StrStr` _array_element "/ModActor.ModActor_C")))))
        (if (`KismetSystemLibrary.IsValid` _returnvalue)
          (if (`KismetSystemLibrary.IsValidClass` (`GameplayStatics.GetObjectClass` _returnvalue))
            (`KismetSystemLibrary.ExecuteConsoleCommand` "enablecheats" null)
            (`KismetSystemLibrary.ExecuteConsoleCommand` (`KismetStringLibrary.Concat_StrStr` "spawnactor " (`KismetStringLibrary.Concat_StrStr` _array_element "/ModActor")) null)))))))

(event `KeyPresses`
  (`/Game/Mods/ModLoader/ModRoot/Shared/BML_Shared.KeyPress` "One"
    (:`Pressed`
      (`self.ToggleModLoaderMenu`))
    (:`Neither`
      ;[1 0.5625 0] Implement Bigger Sub Menus Later On
      (`/Game/Mods/ModLoader/ModRoot/Shared/BML_Shared.KeyPress` "Two"
        (:`Pressed`
          (`self.WBP_ModLoader`
            (:`then`
              (if (`|EnumEquality` "NewEnumerator0" (`/Game/Mods/ModLoader/ModRoot/Modules/ModLoader/WBP_ModLoader.E_CurrentSlideState` (`self.WBP_ModLoader`)))
                (`/Game/Mods/ModLoader/ModRoot/Modules/ModLoader/WBP_ModLoader.SetMenuState` (`self.WBP_ModLoader`) "NewEnumerator1")
                (else
                  (`/Game/Mods/ModLoader/ModRoot/Modules/ModLoader/WBP_ModLoader.SetMenuState` (`self.WBP_ModLoader`) "NewEnumerator0"))))
            (:`else`)))))))

(event `self.ReceiveTick`
  (params (DeltaSeconds :type "Float (single-precision)"))
  (`self.KeyPresses`))

(event `ConstructionTesting`
  (`self.ToggleModLoaderMenu`)
  (`KismetSystemLibrary.Delay` 0.1)
  (`self.ToggleModLoaderMenu`)
  (`self.LoadSave`)
  (`self.PopulateModLoaderInformation`)
  (`self.SaveSave`)
  (`self.GetModLoaderReference`)
  (`self.SpawnMods`)
  (`self.ToggleModLoaderMenu`)
  (`KismetSystemLibrary.Delay` 0.1)
  (`self.ToggleModLoaderMenu`)
  (`Widget.RemoveFromParent` (`self.WBP_ModLoader`)))

(event `PopulateModLoaderInformation`
  ;[1 0.1172 0] Scans Asset Registry For New Content
  (if (`self.bHasLastScanFinished`)
    (set `self.bHasLastScanFinished` false)
    (set `self.BeforeScanDataTables` (`AssetRegistry.GetAssetsByClass` (`AssetRegistryHelpers.GetAssetRegistry`) "DataTable" true))
    (`AssetRegistry.ScanPathsSynchronous` (`AssetRegistryHelpers.GetAssetRegistry`) (`|MakeArray` "/Game/Mods") true)
    (`/Game/Mods/ModLoader/ModRoot/Shared/BML_Shared.WaitUntilAssetRegistryLoaded`
      (:`FinishedLoading`
        (bind _returnvalue (`KismetSystemLibrary.LoadAsset_Blocking` (`self.DT_ModLoadingTypes`)))
        (bind _asdata_table (cast `DataTable` _returnvalue))
        (bind _outrownames (`DataTableFunctionLibrary.GetDataTableRowNames` _asdata_table))
        (for _array_element _outrownames
          (bind _returnvalue_2 (`|GetDataTableRow` _asdata_table _array_element)
            (:`then`
              (bind (_spawnmethod _namingconvention _getobjectstospawnmethod _assetregistrymethod _bisrowinuse) (break `/Game/Mods/ModLoader/ModRoot/Modules/ModLoader/ModLoadingTypes/F_LoadingTypes` _returnvalue_2))
              (if _bisrowinuse
                (switch `/Game/Mods/ModLoader/ModRoot/Modules/ModLoader/ModLoadingTypes/E_GetObjectsToSpawnMethods` _getobjectstospawnmethod
                  (:`NewEnumerator0`
                    (switch `/Game/Mods/ModLoader/ModRoot/Modules/ModLoader/ModLoadingTypes/E_AssetRegistryMethods` _assetregistrymethod
                      (:`NewEnumerator2`
                        (switch `/Game/Mods/ModLoader/ModRoot/Modules/ModLoader/ModLoadingTypes/E_SpawnMethods` _spawnmethod
                          (:`NewEnumerator8`
                            (`self.ModLoading_DA_PDA`))))
                      (:`NewEnumerator0`
                        (switch `/Game/Mods/ModLoader/ModRoot/Modules/ModLoader/ModLoadingTypes/E_SpawnMethods` _spawnmethod
                          (:`NewEnumerator8`
                            (`self.DataTableScanLogic`))))
                      (:`NewEnumerator5`
                        (switch `/Game/Mods/ModLoader/ModRoot/Modules/ModLoader/ModLoadingTypes/E_NamingConventions` _namingconvention
                          (:`NewEnumerator0`
                            (switch `/Game/Mods/ModLoader/ModRoot/Modules/ModLoader/ModLoadingTypes/E_SpawnMethods` _spawnmethod
                              (:`NewEnumerator0`
                                (`self.SpawnLogicModsLevelStreamMethod`))
                              (:`NewEnumerator1`
                                (`self.SpawnLogicModsSpawnActorMethodSummon`))
                              (:`NewEnumerator2`
                                (`self.SpawnLogicModsSpawnActorMethodSpawnActor`))
                              (:`NewEnumerator8`
                                (`self.ModActorScanLogic`)))))))))))))))))

(event `SpawnMods`
  ;[1 0.7031 0] Should eventually only spawn when true, change this later when working on the toggle button functionality
  (bind (_arrayindex _arrayelement) (`/Engine/EditorBlueprintResources/StandardMacros.ReverseForEachLoop` (`self.ModLoaderInformation`))
    (:`LoopBody`
      (bind (_modname _modauthors _modcredits _moddescription _modversion _modbuttons _modclass _spawnedmodactor _bismodactive _modpackagepath _modassetdirectoryname _modinstructions _bdestroyedattachedactors _actorgarbagelist_destroyattachedactors _modmenus_modmenuactive _modqueuepriorityoriginal _modqueuepriorityoverride _busemodqueuepriorityoverride) (break `/Game/Mods/ModLoader/ModRoot/Modules/ModLoader/F_ModLoaderInformation` _arrayelement))
      (if _bismodactive
        _
        (else
          _))
      (bind _returnvalue (`|SpawnActorFromClass` _modclass (`KismetMathLibrary.MakeTransform` (0.0 0.0 0.0)) "AdjustIfPossibleButAlwaysSpawn" "OverrideRootScale" null null))
      (bind _asbp_m_mod_actor (cast `/Game/Mods/ModLoader/ModRoot/Shared/Bases/BP_M_ModActor` _returnvalue))
      (bind (_modbuttons_2 _modqueuepriorityoriginal_2 _bdestroyattachedactors _actorgarbagelist_destroyattachedactors_2 _modmenus_modmenuactive_2) (break `/Game/Mods/ModLoader/ModRoot/Modules/ModLoader/F_ModLoaderModActor` (`/Game/Mods/ModLoader/ModRoot/Shared/Bases/BP_M_ModActor.ModActorInformation` _asbp_m_mod_actor)))
      (bind _output_get (set `/Game/Mods/ModLoader/ModRoot/Shared/Bases/BP_M_ModActor.ModLoaderInformation` (make `/Game/Mods/ModLoader/ModRoot/Modules/ModLoader/F_ModLoaderInformation` _modname _modauthors _modcredits _moddescription _modversion _modbuttons_2 _modclass _returnvalue _bismodactive _modpackagepath _modassetdirectoryname _modinstructions _bdestroyattachedactors _actorgarbagelist_destroyattachedactors_2 _modmenus_modmenuactive_2 _modqueuepriorityoriginal_2 _modqueuepriorityoverride _busemodqueuepriorityoverride) _asbp_m_mod_actor))
      (`KismetArrayLibrary.Array_RemoveItem` (`self.ModLoaderInformation`) _arrayelement)
      (`KismetArrayLibrary.Array_AddUnique` (`self.ModLoaderInformation`) _output_get))))

(fn `ActivateConsole`)

(fn `DataTableScanLogic`
  (locals (DataTableOutRow :type "/Game/Mods/ModLoader/ModRoot/Modules/ModLoader/F_ModLoaderDataTable Structure"))
  (bind (_modclasshard _modname _modauthors _moddescription _modversion _modinstructions _modcredits) (break `/Game/Mods/ModLoader/ModRoot/Modules/ModLoader/F_ModLoaderDataTable` (`local.DataTableOutRow`)))
  (bind (_modclasshard_2 _modname_2 _modauthors_2 _moddescription_2 _modversion_2 _modinstructions_2 _modcredits_2) (break `/Game/Mods/ModLoader/ModRoot/Modules/ModLoader/F_ModLoaderDataTable` (`local.DataTableOutRow`)))
  (set `self.AfterScanDataTableList` (`AssetRegistry.GetAssetsByClass` (`AssetRegistryHelpers.GetAssetRegistry`) "DataTable" true))
  (for _array_element (`self.AfterScanDataTableList`)
    (bind _asdata_table (cast `DataTable` (`AssetRegistryHelpers.GetAsset` _array_element)))
    (bind _outrownames (`DataTableFunctionLibrary.GetDataTableRowNames` _asdata_table))
    (for _array_element_2 _outrownames
      (bind _returnvalue (`|GetDataTableRow` _asdata_table _array_element_2)
        (:`then`
          (set `local.DataTableOutRow` _returnvalue)
          (bind _asbp_m_mod_actor (castclass `/Game/Mods/ModLoader/ModRoot/Shared/Bases/BP_M_ModActor` (`.ModClassHard_28_99B235604F6BD15CE11D18BB5379067A` (break `/Game/Mods/ModLoader/ModRoot/Modules/ModLoader/F_ModLoaderDataTable` (`local.DataTableOutRow`)))))
          (set `self.bIsAlreadyInList` false)
          (for _array_element_3 (`self.SaveModLoaderInformation`)
            (bind (_modclass _bismodactive _busemodqueuepriorityoverride _modqueuepriorityoverride _modmenus_modmenuactive) (break `/Game/Mods/ModLoader/ModRoot/Modules/ModLoader/F_ModLoaderSaveData` _array_element_3))
            (if (== _modclass _modclasshard)
              (set `self.bIsAlreadyInList` true)
              (break)))
          (if (`self.bIsAlreadyInList`)
            (bind (_modbuttons _modqueuepriorityoriginal _bdestroyattachedactors _actorgarbagelist_destroyattachedactors) (break `/Game/Mods/ModLoader/ModRoot/Modules/ModLoader/F_ModLoaderModActor` (`.ModActorInformation` (defaults `/Game/Mods/ModLoader/ModRoot/Modules/ModLoader/BP_ModLoader` _asbp_m_mod_actor))))
            (`KismetArrayLibrary.Array_AddUnique` (`self.ModLoaderInformation`) (make `/Game/Mods/ModLoader/ModRoot/Modules/ModLoader/F_ModLoaderInformation` _modname _modauthors _modcredits _moddescription _modversion _modbuttons _modclasshard null _bismodactive "" "" _modinstructions _bdestroyattachedactors _actorgarbagelist_destroyattachedactors _modmenus_modmenuactive _modqueuepriorityoriginal _modqueuepriorityoverride _busemodqueuepriorityoverride))
            (else
              (bind (_modbuttons_2 _modqueuepriorityoriginal_2 _bdestroyattachedactors_2 _actorgarbagelist_destroyattachedactors_2 _modmenus_modmenuactive_2) (break `/Game/Mods/ModLoader/ModRoot/Modules/ModLoader/F_ModLoaderModActor` (`.ModActorInformation` (defaults `/Game/Mods/ModLoader/ModRoot/Modules/ModLoader/BP_ModLoader` _asbp_m_mod_actor))))
              (`KismetArrayLibrary.Array_AddUnique` (`self.ModLoaderInformation`) (make `/Game/Mods/ModLoader/ModRoot/Modules/ModLoader/F_ModLoaderInformation` _modname_2 _modauthors_2 _modcredits_2 _moddescription_2 _modversion_2 _modbuttons_2 _modclasshard_2 null false "" "" _modinstructions_2 _bdestroyattachedactors_2 _actorgarbagelist_destroyattachedactors_2 _modmenus_modmenuactive_2 _modqueuepriorityoriginal_2))))))))
  (`self.ModListCleanup`)
  (set `self.bHasLastScanFinished` true))

(fn `GetModLoaderReference`
  (`self.WBP_ModLoader`
    (:`then`)
    (:`else`
      (bind _foundwidgets (`WidgetBlueprintLibrary.GetAllWidgetsOfClass` "/Game/Mods/ModLoader/ModRoot/Modules/ModLoader/WBP_ModLoader.WBP_ModLoader_C" false))
      (bind _output (`|GetArrayItem` _foundwidgets))
      (if (not (`KismetSystemLibrary.IsValid` _output))
        (bind _returnvalue (`|CreateWidget` "/Game/Mods/ModLoader/ModRoot/Modules/ModLoader/WBP_ModLoader.WBP_ModLoader_C" null self))
        (set `self.WBP_ModLoader` _returnvalue)
        (else
          (set `self.WBP_ModLoader` _output))))))

(fn `LoadSave`
  (bind _returnvalue (`GameplayStatics.DoesSaveGameExist` (`self.SaveSlotString`)))
  (if _returnvalue
    (bind _returnvalue_2 (`GameplayStatics.LoadGameFromSlot` (`self.SaveSlotString`)))
    (bind _assg_mod_tracker (cast `/Game/Mods/ModLoader/ModRoot/Modules/ModLoader/SG_ModTracker` _returnvalue_2))
    (set `self.SaveGame` _assg_mod_tracker)
    (else
      (bind _returnvalue_3 (`GameplayStatics.CreateSaveGameObject` "/Game/Mods/ModLoader/ModRoot/Modules/ModLoader/SG_ModTracker.SG_ModTracker_C"))
      (bind _output_get (set `self.SaveGame` _returnvalue_3))
      (`GameplayStatics.SaveGameToSlot` _output_get (`self.SaveSlotString`))))
  (set `self.SaveModLoaderInformation` (`/Game/Mods/ModLoader/ModRoot/Modules/ModLoader/SG_ModTracker.ModLoaderInformation` (`self.SaveGame`))))

(fn `ModActorScanLogic`
  ;[0.7813 0 1] Check Asset Registry For Mod Actors, This Method Only Works On Newer Versions, Atleast Not on 4.22
  (for _array_element (`AssetRegistry.GetAllAssets` (`AssetRegistryHelpers.GetAssetRegistry`) true)
    (bind (_objectpath _packagename _packagepath _assetname) (break `AssetData` _array_element))
    (if (`KismetStringLibrary.EqualEqual_StrStr` "ModActor_C" (`KismetStringLibrary.Conv_NameToString` _assetname))
      (bind _returnvalue (`KismetStringLibrary.Conv_NameToString` _packagepath))
      (bind _returnvalue_2 (`KismetSystemLibrary.LoadAsset_Blocking` (`KismetSystemLibrary.Conv_SoftObjPathToSoftObjRef` (`KismetSystemLibrary.MakeSoftObjectPath` (`KismetStringLibrary.Concat_StrStr` _returnvalue "/ModActor.ModActor_C")))))
      (bind _asactor (castclass `Actor` (`GameplayStatics.GetObjectClass` _returnvalue_2)))
      (bind _asbp_m_mod_actor (cast `/Game/Mods/ModLoader/ModRoot/Shared/Bases/BP_M_ModActor` _returnvalue_2))
      (bind (_modname _modauthors _modcredits _moddescription _modversion _modbuttons _modclass _spawnedmodactor _bismodactive _modpackagepath _modassetdirectoryname _modinstructions _bdestroyedattachedactors _actorgarbagelist_destroyattachedactors _modmenus_modmenuactive _modqueuepriorityoriginal _modqueuepriorityoverride _busemodqueuepriorityoverride) (break `/Game/Mods/ModLoader/ModRoot/Modules/ModLoader/F_ModLoaderInformation` (`/Game/Mods/ModLoader/ModRoot/Shared/Bases/BP_M_ModActor.ModLoaderInformation` _asbp_m_mod_actor)))
      (`KismetArrayLibrary.Array_AddUnique` (`self.ModLoaderInformation`) (make `/Game/Mods/ModLoader/ModRoot/Modules/ModLoader/F_ModLoaderInformation` _modname _modauthors _modcredits _moddescription _modversion _modbuttons _asactor _spawnedmodactor _bismodactive _returnvalue (`KismetStringLibrary.RightChop` _returnvalue 11) _modinstructions _bdestroyedattachedactors _actorgarbagelist_destroyattachedactors _modmenus_modmenuactive _modqueuepriorityoriginal _modqueuepriorityoverride _busemodqueuepriorityoverride))))
  (`self.ModListCleanup`)
  (set `self.bHasLastScanFinished` true))

(fn `ModListCleanup`
  (bind (_arrayindex _arrayelement) (`/Engine/EditorBlueprintResources/StandardMacros.ReverseForEachLoop` (`self.ModLoaderInformation`))
    (:`LoopBody`
      (if (not (`KismetSystemLibrary.IsValidClass` (`.ModClass_19_9BAD26184531C59D8D667BBC870BBEAB` (break `/Game/Mods/ModLoader/ModRoot/Modules/ModLoader/F_ModLoaderInformation` _arrayelement))))
        (`KismetArrayLibrary.Array_RemoveItem` (`self.ModLoaderInformation`) _arrayelement)))
    (:`Completed`
      ;[1 0 0.4687] Comment
      (`self.SaveSave`))))

(fn `ModLoading_DA_PDA`
  (locals (DataTableOutRow :type "/Game/Mods/ModLoader/ModRoot/Modules/ModLoader/F_ModLoaderDataTable Structure"))
  (bind (_modclasshard _modname _modauthors _moddescription _modversion _modinstructions _modcredits) (break `/Game/Mods/ModLoader/ModRoot/Modules/ModLoader/F_ModLoaderDataTable` (`local.DataTableOutRow`)))
  (bind (_modclasshard_2 _modname_2 _modauthors_2 _moddescription_2 _modversion_2 _modinstructions_2 _modcredits_2) (break `/Game/Mods/ModLoader/ModRoot/Modules/ModLoader/F_ModLoaderDataTable` (`local.DataTableOutRow`)))
  (for _array_element (`AssetRegistry.GetAssetsByClass` (`AssetRegistryHelpers.GetAssetRegistry`) "PrimaryDataAsset" true)
    (bind _aspda_mod_loader (cast `/Game/Mods/ModLoader/ModRoot/Shared/Bases/PDA_ModLoader` (`AssetRegistryHelpers.GetAsset` _array_element)))
    (for _array_element_2 (`/Game/Mods/ModLoader/ModRoot/Shared/Bases/PDA_ModLoader.ModLoaderInformation` _aspda_mod_loader)
      (set `local.DataTableOutRow` _array_element_2)
      (bind _asbp_m_mod_actor (castclass `/Game/Mods/ModLoader/ModRoot/Shared/Bases/BP_M_ModActor` (`.ModClassHard_28_99B235604F6BD15CE11D18BB5379067A` (break `/Game/Mods/ModLoader/ModRoot/Modules/ModLoader/F_ModLoaderDataTable` (`local.DataTableOutRow`)))))
      (set `self.bIsAlreadyInList` false)
      (for _array_element_3 (`self.SaveModLoaderInformation`)
        (bind (_modclass _bismodactive _busemodqueuepriorityoverride _modqueuepriorityoverride _modmenus_modmenuactive) (break `/Game/Mods/ModLoader/ModRoot/Modules/ModLoader/F_ModLoaderSaveData` _array_element_3))
        (if (== _modclass _modclasshard)
          (set `self.bIsAlreadyInList` true)
          (break)))
      (if (`self.bIsAlreadyInList`)
        (bind (_modbuttons _modqueuepriorityoriginal _bdestroyattachedactors _actorgarbagelist_destroyattachedactors) (break `/Game/Mods/ModLoader/ModRoot/Modules/ModLoader/F_ModLoaderModActor` (`.ModActorInformation` (defaults `/Game/Mods/ModLoader/ModRoot/Modules/ModLoader/BP_ModLoader` _asbp_m_mod_actor))))
        (`KismetArrayLibrary.Array_AddUnique` (`self.ModLoaderInformation`) (make `/Game/Mods/ModLoader/ModRoot/Modules/ModLoader/F_ModLoaderInformation` _modname _modauthors _modcredits _moddescription _modversion _modbuttons _modclasshard null _bismodactive "" "" _modinstructions _bdestroyattachedactors _actorgarbagelist_destroyattachedactors _modmenus_modmenuactive _modqueuepriorityoriginal _modqueuepriorityoverride _busemodqueuepriorityoverride))
        (else
          (bind (_modbuttons_2 _modqueuepriorityoriginal_2 _bdestroyattachedactors_2 _actorgarbagelist_destroyattachedactors_2 _modmenus_modmenuactive_2) (break `/Game/Mods/ModLoader/ModRoot/Modules/ModLoader/F_ModLoaderModActor` (`.ModActorInformation` (defaults `/Game/Mods/ModLoader/ModRoot/Modules/ModLoader/BP_ModLoader` _asbp_m_mod_actor))))
          (`KismetArrayLibrary.Array_AddUnique` (`self.ModLoaderInformation`) (make `/Game/Mods/ModLoader/ModRoot/Modules/ModLoader/F_ModLoaderInformation` _modname_2 _modauthors_2 _modcredits_2 _moddescription_2 _modversion_2 _modbuttons_2 _modclasshard_2 null false "" "" _modinstructions_2 _bdestroyattachedactors_2 _actorgarbagelist_destroyattachedactors_2 _modmenus_modmenuactive_2 _modqueuepriorityoriginal_2))))))
  (`self.ModListCleanup`)
  (set `self.bHasLastScanFinished` true))

(fn `SaveSave`
  (set `/Game/Mods/ModLoader/ModRoot/Modules/ModLoader/SG_ModTracker.ModLoaderInformation` (`self.SaveModLoaderInformation`) (`self.SaveGame`))
  (`GameplayStatics.SaveGameToSlot` (`self.SaveGame`) (`self.SaveSlotString`)))

(fn `ToggleModLoaderMenu`
  (if (`KismetSystemLibrary.IsValid` (`self.WBP_ModLoader`))
    (if (`Widget.IsInViewport` (`self.WBP_ModLoader`))
      (`/Game/Mods/ModLoader/ModRoot/Modules/ModLoader/WBP_ModLoader.SetMenuState` (`self.WBP_ModLoader`) "NewEnumerator2")
      (else
        (`UserWidget.AddToViewport` (`self.WBP_ModLoader`) 99)
        (set `self.bOriginalCursorState` (`PlayerController.bShowMouseCursor` (`GameplayStatics.GetPlayerController` 0)))
        (set `PlayerController.bShowMouseCursor` true (`GameplayStatics.GetPlayerController` 0))
        (`WidgetBlueprintLibrary.SetInputMode_GameAndUIEx` (`GameplayStatics.GetPlayerController` 0) (`self.WBP_ModLoader`) "LockAlways" false)))))

(fn `UserConstructionScript`
  (`self.ConstructionTesting`))