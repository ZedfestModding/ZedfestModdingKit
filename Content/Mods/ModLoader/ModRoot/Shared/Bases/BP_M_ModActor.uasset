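; BP_M_ModActor is a base actor for mods that registers a mod's menus in the mod loader UI.
; On BeginPlay it polls with a short delay until WBP_ModLoader exists, then walks the active menu classes in ModActorInformation.
; It re-adds matching existing WBP_Main_Entry widgets to the loader's list when that menu is already instantiated, otherwise creates new entries labeled with the mod name.
; ModButtonWasPressed is an empty stub.
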(event `self.ReceiveBeginPlay`
  (bind (_modbuttons _modqueuepriorityoriginal _bdestroyattachedactors _actorgarbagelist_destroyattachedactors _modmenus_modmenuactive) (break `/Game/Mods/ModLoader/ModRoot/Modules/ModLoader/F_ModLoaderModActor` (`self.ModActorInformation`)))
  (bind _returnvalue (`KismetTextLibrary.Conv_StringToText` (`.ModName_2_508F97D64480667C0B029280456ECDF8` (break `/Game/Mods/ModLoader/ModRoot/Modules/ModLoader/F_ModLoaderInformation` (`self.ModLoaderInformation`)))))
  (bind _foundwidgets (`WidgetBlueprintLibrary.GetAllWidgetsOfClass` "/Game/Mods/ModLoader/ModRoot/Modules/ModLoader/WBP_ModLoader.WBP_ModLoader_C" false :!label _label))
  (if (not (`KismetSystemLibrary.IsValid` (`|GetArrayItem` _foundwidgets)))
    (`KismetSystemLibrary.Delay` 0.05)
    (goto _label)
    (else
      (bind _keys (`BlueprintMapLibrary.Map_Keys` _modmenus_modmenuactive))
      (for _array_element _keys
        (bind (_value _returnvalue_2) (`BlueprintMapLibrary.Map_Find` _modmenus_modmenuactive _array_element))
        (if _returnvalue_2
          (if _value
            (bind _foundwidgets_2 (`WidgetBlueprintLibrary.GetAllWidgetsOfClass` _array_element false))
            (set `self.bPassed` false)
            (for _array_element_2 _foundwidgets_2
              (if (`KismetSystemLibrary.IsValid` _array_element_2)
                (set `self.bPassed` true)
                (break)))
            (if (`self.bPassed`)
              (bind _foundwidgets_3 (`WidgetBlueprintLibrary.GetAllWidgetsOfClass` "/Game/Mods/ModLoader/ModRoot/Modules/ModLoader/WBP_Main_Entry.WBP_Main_Entry_C" false))
              (for _array_element_3 _foundwidgets_3
                (if (== (`/Game/Mods/ModLoader/ModRoot/Modules/ModLoader/WBP_Main_Entry.MainMenuClass` _array_element_3) _array_element)
                  (if (`KismetTextLibrary.EqualEqual_TextText` (`/Game/Mods/ModLoader/ModRoot/Modules/ModLoader/WBP_Main_Entry.ModMenuTextLabel` _array_element_3) _returnvalue)
                    (bind _listview_57 (`/Game/Mods/ModLoader/ModRoot/Modules/ModLoader/WBP_ModLoader.ListView_57` (`|GetArrayItem` _foundwidgets)))
                    (`ListView.AddItem` _listview_57 _array_element_3)
                    (`ListView.AddItem` (`/Game/Mods/ModLoader/ModRoot/Modules/ModLoader/WBP_ModLoader.ListView_57` (`|GetArrayItem` _foundwidgets)) _array_element_3)
                    (break))))
              (else
                (bind _returnvalue_3 (`|CreateWidget` "/Game/Mods/ModLoader/ModRoot/Modules/ModLoader/WBP_Main_Entry.WBP_Main_Entry_C" null _returnvalue _array_element))
                (`ListView.AddItem` _listview_57 _returnvalue_3)))))))))

(fn `ModButtonWasPressed`
  (params (FunctionIndex :type Integer)))

(fn `UserConstructionScript`)